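; Game mode for a rock-paper-scissors gambling match between Player and Computer, running timed rounds and settling the stakes.
; A timer ends each round and broadcasts the result; ties trigger a delayed reset event, while wins move balance from loser to winner.
; A loss with a played hand opens the Stranded minigame, switching camera and crosshair.
; Winning it pays the player half the reward; losing doubles the penalty.
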(event `self.ReceiveBeginPlay`
  (add `self.OnRoundConclude` (delegate `RoundConcluded`))
  (`KismetSystemLibrary.Delay` 0.2)
  (`self.BeginRound`))

(event `RoundConcluded` :!signature `self.OnRoundConclude`
  (params (Winner :type "EParticipant Enum" :default "None") (Tie :type Boolean) (Redeemable :type Boolean))
  (if Tie
    (`KismetSystemLibrary.Delay` 2.0)
    (`self.ResetRound`)
    (else
      (switch `EParticipant` Winner
        (:`Player`
          (`self.DealReward` (`self.Reward`) "Player"))
        (:`Computer`
          (if Redeemable
            (bind _returnvalue (`self.GetMinigameManager`)
              (:`True`
                (bind (_success _returnvalue_2) (`MinigameManager.BeginMinigame` _returnvalue "Stranded"))
                (bind _returnvalue_3 (`self.GetCameraManager`)
                  (:`True`
                    (`CameraManager.ChangeCamera` _returnvalue_3 "Stranded")
                    (if _success
                      (add `Minigame.OnMinigameEnd` _returnvalue_2 (delegate `MinigameEnd`))
                      (bind _returnvalue_4 (`self.GetGamblerController`)
                        (:`True`
                          (`GamblerController.UpdateCrosshairTexture` _returnvalue_4 "Crosshair"))))))))
            (else
              (`self.DealReward` (`self.Reward`) "Computer"))))))))

(event `MinigameEnd`
  (params (bWin :type Boolean))
  (bind _returnvalue (`self.GetCameraManager`)
    (:`True`
      (`CameraManager.ChangeCamera` _returnvalue "Default")
      (bind _returnvalue_2 (`self.GetGamblerController`)
        (:`True`
          (`GamblerController.UpdateCrosshairTexture` _returnvalue_2 "Default")
          (if bWin
            (`self.DealReward` (/ (`self.Reward`) 2.0) "Player")
            (else
              (`self.DealReward` (* (`self.Reward`) 2.0) "Computer"))))))))

(event `BeginRound`
  (if (not (`self.RoundActive`))
    (`self.ResetHands`)
    (`self.OnRoundBegin`)
    (bind _returnvalue (`KismetSystemLibrary.K2_SetTimerDelegate` (delegate `ConcludeRound`) (`self.RoundDuration`)))
    (set `self.RoundTimerHandle` _returnvalue)
    (set `self.RoundActive` true)))

(event `ConcludeRound`
  (`KismetSystemLibrary.K2_ClearAndInvalidateTimerHandle` (`self.RoundTimerHandle`))
  (set `self.RoundActive` false)
  (bind (_winner _tie) (`self.GetWinner`))
  (`self.OnRoundConclude` _winner _tie (`self.HasPlayedHand` "Player")))

(event `ResetRound`
  (`self.OnRoundReset`))

(fn `DealReward`
  (params (Amount :type "Float (double-precision)") (Winner :type "EParticipant Enum" :default "None"))
  (locals (Loser :type "EParticipant Enum"))
  (`|ExecutionSequence`
    (:`then_0`
      (switch `EParticipant` Winner
        (:`Player`
          (set `local.Loser` "Computer"))
        (:`Computer`
          (set `local.Loser` "Player"))))
    (:`then_1`
      (bind _returnvalue (`self.GetParticipantManager`)
        (:`True`
          (bind _returnvalue_2 (`ParticipantManager.GetParticipant` _returnvalue (`local.Winner`))
            (:`True`
              (bind _returnvalue_3 (`UtilityBlueprintFunctionLibrary.HasParticipantComponent` _returnvalue_2)
                (:`True`
                  (`ParticipantComponent.AddBalance` _returnvalue_3 (`local.Amount`)))))))))
    (:`then_2`
      (bind _returnvalue_4 (`self.GetParticipantManager`)
        (:`True`
          (bind _returnvalue_5 (`ParticipantManager.GetParticipant` _returnvalue_4 (`local.Loser`))
            (:`True`
              (bind _returnvalue_6 (`UtilityBlueprintFunctionLibrary.HasParticipantComponent` _returnvalue_5)
                (:`True`
                  (`ParticipantComponent.SubtractBalance` _returnvalue_6 (`local.Amount`)))))))))))

(fn `UserConstructionScript`)