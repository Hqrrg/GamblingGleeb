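; BP_Gambler is a rock-paper-scissors participant that displays its hand as a flipbook, driven by round events from BP_RPSGameMode.
; On round begin it shows the PF_RPS flipbook, plays a hard-coded Scissors hand for the Player participant and prints a debug message.
; On conclusion it looks up its own participant's hand in the HandFlipbooks map to update the display; reset uses the None entry.
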(event `self.ReceiveBeginPlay`
  (bind _asbp_rpsgame_mode (cast `/Game/GamblingGleeb/Core/BP_RPSGameMode` (`GameplayStatics.GetGameMode`)))
  (bind _output_get (set `self.RPSGameMode` _asbp_rpsgame_mode))
  (add `/Game/GamblingGleeb/Core/BP_RPSGameMode.OnRoundBegin` _output_get (delegate `RoundBegin`))
  (add `/Game/GamblingGleeb/Core/BP_RPSGameMode.OnRoundConclude` (`self.RPSGameMode`) (delegate `RoundConcluded`))
  (add `/Game/GamblingGleeb/Core/BP_RPSGameMode.OnRoundReset` (`self.RPSGameMode`) (delegate `RoundReset`)))

(event `RoundConcluded`
  (params (Winner :type "EParticipant Enum" :default "None") (Tie :type Boolean) (Redeemable :type Boolean))
  (`self.UpdateHandFlipbook` (`RPSGameMode.GetHand` (`self.RPSGameMode`) (`ParticipantComponent.GetParticipantKey` (`self.Participant`)))))

(event `RoundBegin`
  (`PaperFlipbookComponent.SetFlipbook` (`self.HandFlipbook`) "/Game/GamblingGleeb/Asset/Flipbooks/PF_RPS.PF_RPS")
  (`RPSGameMode.PlayHand` (`self.RPSGameMode`) "Player" "Scissors")
  (`KismetSystemLibrary.PrintString` "Hello"))

(event `RoundReset`
  (`self.UpdateHandFlipbook` "None"))

(event `UpdateHandFlipbook`
  (params (Key :type "EHand Enum" :default "None"))
  (bind (_value _returnvalue) (`BlueprintMapLibrary.Map_Find` (`self.HandFlipbooks`) Key))
  ;[1 1 1] Update the hand flipbook
  (if _returnvalue
    (`PaperFlipbookComponent.SetFlipbook` (`self.HandFlipbook`) _value)))

(fn `UserConstructionScript`)