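; BP_Gleeb is a rock-paper-scissors gambling participant that plays random hands and shows them with flipbooks.
; It binds to BP_RPSGameMode round events, submitting a random hand under its participant key as a round begins while displaying the RPS flipbook.
; At conclusion it reveals that hand through a flipbook map lookup, and round reset applies the None entry.
; When its balance runs out, it ends the game through the game mode.
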(event `self.ReceiveBeginPlay`
  (bind _asbp_rpsgame_mode (cast `/Game/GamblingGleeb/Core/BP_RPSGameMode` (`GameplayStatics.GetGameMode`)))
  (bind _output_get (set `self.RPSGameMode` _asbp_rpsgame_mode))
  (add `/Game/GamblingGleeb/Core/BP_RPSGameMode.OnRoundBegin` _output_get (delegate `RoundStarted`))
  (add `/Game/GamblingGleeb/Core/BP_RPSGameMode.OnRoundConclude` (`self.RPSGameMode`) (delegate `RoundConcluded`))
  (add `/Game/GamblingGleeb/Core/BP_RPSGameMode.OnRoundReset` (`self.RPSGameMode`) (delegate `RoundReset`)))

(event `RoundConcluded`
  (params (Winner :type "EParticipant Enum" :default "None") (Tie :type Boolean) (Redeemable :type Boolean))
  (`self.UpdateHandFlipbook` (`RPSGameMode.GetHand` (`self.RPSGameMode`) (`ParticipantComponent.GetParticipantKey` (`self.Participant`)))))

(event `RoundStarted`
  (`PaperFlipbookComponent.SetFlipbook` (`self.HandFlipbook`) (`self.RPSFlipbook`))
  (`RPSGameMode.PlayHand` (`self.RPSGameMode`) (`ParticipantComponent.GetParticipantKey` (`self.Participant`)) (`self.GetRandomHand`)))

(event `RoundReset`
  (`self.UpdateHandFlipbook` "None"))

(event `UpdateHandFlipbook`
  (params (Key :type "EHand Enum" :default "None"))
  (bind (_value _returnvalue) (`BlueprintMapLibrary.Map_Find` (`self.HandFlipbooks`) Key))
  ;[1 1 1] Update the RPS flipbook
  (if _returnvalue
    (`PaperFlipbookComponent.SetFlipbook` (`self.HandFlipbook`) _value)))

(event `self.Participant.OnBalanceUpdated`
  (params (Balance :type "Float (single-precision)"))
  (bind _rpsgamemode (`self.RPSGameMode`))
  (if (<= Balance 0.0)
    (`/Engine/EditorBlueprintResources/StandardMacros.IsValid` _rpsgamemode
      (:`Is Valid`
        (`/Game/GamblingGleeb/Core/BP_RPSGameMode.EndGame` _rpsgamemode true)))))

(fn `GetRandomHand`
  (returns (Hand :type "EHand Enum"))
  (locals (NewLocalVar :type "EHand Enum"))
  (return (select `int` (`KismetMathLibrary.RandomIntegerInRange` 0 2) :`0` "Rock" :`1` "Paper" :`2` "Scissors" :!type "EHand Enum")))

(fn `UserConstructionScript`)