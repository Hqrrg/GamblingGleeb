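; BP_Bank is an in-world display that shows a game participant's balance as pound-prefixed text.
; On BeginPlay it waits for the RPS game mode's managers-loaded event, then looks up its assigned participant through the participant manager.
; It binds to that participant component's balance-updated event and writes each new balance, truncated to a whole number, to its TextRender.
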(event `self.ReceiveBeginPlay`
  (bind _asbp_rpsgame_mode (cast `/Game/GamblingGleeb/Core/BP_RPSGameMode` (`GameplayStatics.GetGameMode`)))
  (bind _output_get (set `self.RPSGameMode` _asbp_rpsgame_mode))
  (add `RPSGameMode.OnManagersLoaded` _output_get (delegate `ManagersLoaded`)))

(event `ManagersLoaded`
  (bind _returnvalue (`RPSGameMode.GetParticipantManager` (`self.RPSGameMode`))
    (:`True`
      (bind _returnvalue_2 (`ParticipantManager.GetParticipant` _returnvalue (`self.Participant`))
        (:`True`
          (bind _returnvalue_3 (`UtilityBlueprintFunctionLibrary.HasParticipantComponent` _returnvalue_2)
            (:`True`
              (add `ParticipantComponent.OnBalanceUpdated` _returnvalue_3 (delegate `BalanceUpdated`)))))))))

(event `BalanceUpdated`
  (params (Balance :type "Float (single-precision)"))
  (`TextRenderComponent.K2_SetText` (`self.TextRender`) (`KismetTextLibrary.Conv_StringToText` (`KismetStringLibrary.Concat_StrStr` "£" (`KismetStringLibrary.Conv_IntToString` (`KismetMathLibrary.FTrunc` Balance))))))

(fn `UserConstructionScript`)